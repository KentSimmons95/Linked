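; BP_LinkedPlayerController is a player controller that toggles the pause menu from the OptionMenu input action.
; When the game is running, a press pauses it, creates and shows WBP_PauseMenu, and switches to UI-only input focused on that menu with the mouse unlocked.
; When the game is paused, a press unpauses it, removes all widgets rather than just the menu, and restores game-only input.
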(event EventBeginPlay)

(event EventTick
  (params (DeltaSeconds :type Float%20%28single-precision%29)))

(event Input|ActionEvents|InputActionOptionMenu
  (params (Key :type Key%20Structure :default "None"))
  (:Pressed
    (if (Game|IsGamePaused)
      (Game|SetGamePaused false)
      (Viewport|RemoveAllWidgets)
      (Input|SetInputModeGameOnly self)
      (else
        (Game|SetGamePaused true)
        (bind _returnvalue (UserInterface|CreateWidget "/Game/UI/WBP_PauseMenu.WBP_PauseMenu_C"))
        (UserInterface|Viewport|AddtoViewport _returnvalue 0)
        (Input|SetInputModeUIOnly self _returnvalue "DoNotLock")))))

(fn ConstructionScript)